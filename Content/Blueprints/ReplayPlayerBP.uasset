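; ReplayPlayerBP is the input layer for controlling replay playback.
; Input actions map directly to calls for pausing, setting playback direction, resetting, single-stepping, and seeking to the previous or next incident.
; A hardcoded F3 key toggles arrow display.
; The graph holds no playback logic of its own, only forwarding presses to functions defined outside it.
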(event Input|ActionEvents|InputActionSeekBackwardsToIncident
  (:Pressed
    (Class|ReplayPlayer|SeektoIncident "PD_Backward")))

(event Input|ActionEvents|InputActionPlaybackReset
  (:Pressed
    (Class|ReplayPlayer|ResetPlayback)))

(event Input|ActionEvents|InputActionStepForward
  (:Pressed
    (Class|ReplayPlayer|Step "PD_Forward")))

(event Input|ActionEvents|InputActionStepBack
  (:Pressed
    (Class|ReplayPlayer|Step "PD_Backward")))

(event Input|ActionEvents|InputActionSeekForwardToIncident
  (:Pressed
    (Class|ReplayPlayer|SeektoIncident "PD_Forward")))

(event Input|ActionEvents|InputActionPlaybackForward
  (:Pressed
    (Class|ReplayPlayer|SetDirection "PD_Forward")))

(event Input|ActionEvents|InputActionPlaybackBackward
  (:Pressed
    (Class|ReplayPlayer|SetDirection "PD_Backward")))

(event Input|ActionEvents|InputActionPausePlayback
  (:Pressed
    (Class|ReplayPlayer|TogglePause)))

(event Input|KeyboardEvents|F3
  (:Pressed
    (Class|ReplayPlayer|ToggleShowArrows)))

(fn ConstructionScript)