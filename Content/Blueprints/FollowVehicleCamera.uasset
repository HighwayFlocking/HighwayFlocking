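; FollowVehicleCamera is a camera actor that turns to follow the replay's current look-at target.
; On BeginPlay it caches the first ReplayPlayerBP found in the level.
; Each tick, if that player's LookAtActor is valid, it rotates to face it, adding DegreesAbove to the pitch as a vertical framing offset.
; It only sets rotation and never changes its own location.
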(event EventBeginPlay
  (bind _outactors (Actor|GetAllActorsOfClass "/Game/Blueprints/ReplayPlayerBP.ReplayPlayerBP_C"))
  (Variables|Default|SetReplayPlayer (Utilities|Array|Get(acopy) _outactors)))

(event EventActorBeginOverlap
  (params (OtherActor :type Actor%20Object%20Reference)))

(event EventTick
  (params (DeltaSeconds :type Float%20%28single-precision%29))
  (bind _returnvalue (Transformation|GetActorLocation))
  (bind _replayplayer (Variables|Default|GetReplayPlayer))
  (bind _lookatactor (Variables|/Script/Vehicle.ReplayPlayer|GetLookAtActor _replayplayer))
  (bind _returnvalue_2 (Transformation|GetActorLocation _lookatactor))
  (bind _returnvalue_3 (Math|Rotator|FindLookatRotation _returnvalue _returnvalue_2))
  (bind (_pitch _yaw _roll) (Class|KismetMathLibrary|BreakRot _returnvalue_3))
  (if (Utilities|IsValid _lookatactor)
    (Transformation|SetActorRotation (Class|KismetMathLibrary|MakeRot (+ _pitch (Variables|Default|GetDegreesAbove)) _yaw _roll))))

(fn ConstructionScript)