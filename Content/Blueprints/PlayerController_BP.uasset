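; Player controller for a vehicle flocking sandbox, providing debug tools to spawn, possess, delete and control cars.
; BeginPlay caches the Roadmap and Behaviours actors and creates a toggleable menu widget fed by Behaviours.
; Camera-forward line traces pick targets for possession, deletion, max-speed toggling and teleporting, and place FlockingCars aligned to the nearest road tangent, optionally reversed.
; Other inputs adjust FOV and toggle HUD visibility and vehicle ID drawing.
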(event EventBeginPlay
  (Utilities|FlowControl|Sequence
    (:then_0
      (bind _outactors (Actor|GetAllActorsOfClass "/Game/Blueprints/Roadmap_BP.Roadmap_BP_C"))
      (Variables|Default|SetRoadmap (Utilities|Array|Get(acopy) _outactors)))
    (:then_1
      (bind _outactors_2 (Actor|GetAllActorsOfClass "/Game/Blueprints/Behaviours_BP.Behaviours_BP_C"))
      (Variables|Default|SetBehaviours (Utilities|Array|Get(acopy) _outactors_2)))
    (:then_2
      (bind _returnvalue (UserInterface|CreateWidget "/Game/UMG/MenuHUD.MenuHUD_C" 0 (Variables|Default|GetBehaviours)))
      (Variables|Default|SetMenuWidget _returnvalue))))

(event Input|ActionEvents|InputActionMenu
  (bind _menuwidget (Variables|Default|GetMenuWidget))
  (:Pressed
    (bind _output_get (Variables|Default|SetMenuShowing (not (Variables|Default|GetMenuShowing))))
    (if _output_get
      (UserInterface|Viewport|AddtoViewport _menuwidget 0)
      (else
        (Widget|RemovefromParent _menuwidget)))
    (bind _output_get_2 (Variables|Default|SetbShowMouseCursor _output_get))
    (Variables|Default|SetbEnableMouseOverEvents _output_get_2)))

(event Input|ActionEvents|InputActionDelete
  (bind _returnvalue (Game|GetPlayerCameraManager 0))
  (bind _returnvalue_2 (Transformation|GetActorLocation _returnvalue))
  (:Pressed
    (bind _outhit (Collision|LineTraceByChannel _returnvalue_2 (+ _returnvalue_2 (* (Math|Vector|Normalize (Math|Rotator|GetRotationXVector (Transformation|GetActorRotation _returnvalue))) 1e+05)) "TraceTypeQuery1" false 0 "None"))
    (bind _aswheeled_vehicle (Utilities|Casting|CastToWheeledVehicle (.HitActor (Collision|BreakHitResult _outhit))))
    (Actor|DestroyActor _aswheeled_vehicle)))

(event Input|ActionEvents|InputActionToggleZeroMaxSpeed
  (bind _returnvalue (Game|GetPlayerCameraManager 0))
  (bind _returnvalue_2 (Transformation|GetActorLocation _returnvalue))
  (:Pressed
    (bind _outhit (Collision|LineTraceByChannel _returnvalue_2 (+ _returnvalue_2 (* (Math|Vector|Normalize (Math|Rotator|GetRotationXVector (Transformation|GetActorRotation _returnvalue))) 1e+05)) "TraceTypeQuery1" false 0 "None"))
    (bind _asflocking_vehicle (Utilities|Casting|CastToFlockingVehicle (.HitActor (Collision|BreakHitResult _outhit))))
    (Math|Float|CompareFloat (Variables|/Script/Vehicle.FlockingVehicle|GetMaxSpeed _asflocking_vehicle) 8e+01
      (:==
        (Variables|/Script/Vehicle.FlockingVehicle|SetMaxSpeed _asflocking_vehicle 0.0))
      (:<
        (Variables|/Script/Vehicle.FlockingVehicle|SetMaxSpeed _asflocking_vehicle 8e+01)))))

(event Input|ActionEvents|InputActionTeleport
  (bind _returnvalue (Game|GetPlayerCameraManager 0))
  (bind _returnvalue_2 (Game|Player|GetPlayerPawn 0))
  (bind _returnvalue_3 (Transformation|GetActorLocation _returnvalue))
  (:Pressed
    (bind _outhit (Collision|LineTraceByChannel _returnvalue_3 (+ _returnvalue_3 (* (Math|Vector|Normalize (Math|Rotator|GetRotationXVector (Transformation|GetActorRotation _returnvalue))) 1e+05)) "TraceTypeQuery1" false 0 "None"))
    (Transformation|Teleport _returnvalue_2 (Math|Vector|MakeVector (.X (Math|Vector|BreakVector (.Location (Collision|BreakHitResult _outhit)))) (.Y (Math|Vector|BreakVector (.Location (Collision|BreakHitResult _outhit)))) (.Z (Math|Vector|BreakVector (Transformation|GetActorLocation _returnvalue_2)))) (Transformation|GetActorRotation _returnvalue_2))))

(event Input|ActionEvents|InputActionSpanGolf
  (bind _returnvalue (Game|GetPlayerCameraManager 0))
  (bind _returnvalue_2 (Transformation|GetActorLocation _returnvalue))
  (:Pressed
    (Variables|Default|SetReversed false)
    (bind _outhit (Collision|LineTraceByChannel _returnvalue_2 (+ _returnvalue_2 (* (Math|Vector|Normalize (Math|Rotator|GetRotationXVector (Transformation|GetActorRotation _returnvalue))) 1e+05)) "TraceTypeQuery1" false 0 "None"))
    (bind _returnvalue_3 (Game|SpawnActorfromClass "/Game/Vehicle/FlockingCar.FlockingCar_C" (Math|Transform|MakeTransform (+ (.Location (Collision|BreakHitResult _outhit)) (* (Math|Vector|GetUpVector "0, 0, 0") 0.0)) (Math|Rotator|MakeRotfromX (select (Variables|Default|GetReversed) (Math|Vector|NegateVector (Class|Roadmap|GetRoadTangentNearest (Variables|Default|GetRoadmap) (.Location (Collision|BreakHitResult _outhit)))) (Class|Roadmap|GetRoadTangentNearest (Variables|Default|GetRoadmap) (.Location (Collision|BreakHitResult _outhit)))))) false 0))
    (Pawn|SpawnDefaultController _returnvalue_3)))

(event Input|ActionEvents|InputActionSpanGolfReversed
  (bind _returnvalue (Game|GetPlayerCameraManager 0))
  (bind _returnvalue_2 (Transformation|GetActorLocation _returnvalue))
  (:Pressed
    (Variables|Default|SetReversed true)
    (bind _outhit (Collision|LineTraceByChannel _returnvalue_2 (+ _returnvalue_2 (* (Math|Vector|Normalize (Math|Rotator|GetRotationXVector (Transformation|GetActorRotation _returnvalue))) 1e+05)) "TraceTypeQuery1" false 0 "None"))
    (bind _returnvalue_3 (Game|SpawnActorfromClass "/Game/Vehicle/FlockingCar.FlockingCar_C" (Math|Transform|MakeTransform (+ (.Location (Collision|BreakHitResult _outhit)) (* (Math|Vector|GetUpVector "0, 0, 0") 0.0)) (Math|Rotator|MakeRotfromX (select (Variables|Default|GetReversed) (Math|Vector|NegateVector (Class|Roadmap|GetRoadTangentNearest (Variables|Default|GetRoadmap) (.Location (Collision|BreakHitResult _outhit)))) (Class|Roadmap|GetRoadTangentNearest (Variables|Default|GetRoadmap) (.Location (Collision|BreakHitResult _outhit)))))) false 0))
    (Pawn|SpawnDefaultController _returnvalue_3)))

(event Input|ActionEvents|InputActionEnterVehicle
  (bind _returnvalue (Game|GetPlayerCameraManager 0))
  (bind _returnvalue_2 (Transformation|GetActorLocation _returnvalue))
  (:Pressed
    (bind _outhit (Collision|LineTraceByChannel _returnvalue_2 (+ _returnvalue_2 (* (Math|Vector|Normalize (Math|Rotator|GetRotationXVector (Transformation|GetActorRotation _returnvalue))) 1e+05)) "TraceTypeQuery1" false 0 "None"))
    (bind _aspawn (Utilities|Casting|CastToPawn (.HitActor (Collision|BreakHitResult _outhit))))
    (Pawn|Possess _aspawn)
    (bind _asmocking_vehicle (Utilities|Casting|CastToMockingVehicle _aspawn))
    (Development|PrintString (Utilities|String|ToString(Integer) (Variables|/Script/Vehicle.MockingVehicle|GetReplayUniqueId _asmocking_vehicle)))))

(event Input|ActionEvents|InputActionFovIN
  (bind _returnvalue (Game|GetPlayerCameraManager 0))
  (:Pressed
    (Variables|/Script/Engine.PlayerCameraManager|SetDefaultFOV _returnvalue (- (Variables|/Script/Engine.PlayerCameraManager|GetDefaultFOV _returnvalue) 1.0))))

(event Input|ActionEvents|InputActionFovOut
  (bind _returnvalue (Game|GetPlayerCameraManager 0))
  (:Pressed
    (Variables|/Script/Engine.PlayerCameraManager|SetDefaultFOV _returnvalue (+ (Variables|/Script/Engine.PlayerCameraManager|GetDefaultFOV _returnvalue) 1.0))))

(event Input|KeyboardEvents|F4
  (:Pressed
    (bind _aschud (Utilities|Casting|CastToCHud (HUD|GetHUD)))
    (Variables|/Script/Vehicle.CHud|SetHideHud _aschud (not (Variables|/Script/Vehicle.CHud|GetHideHud _aschud)))))

(event Input|KeyboardEvents|F6
  (:Pressed
    (bind _aschud (Utilities|Casting|CastToCHud (HUD|GetHUD)))
    (Variables|/Script/Vehicle.CHud|SetDrawVehicleIds _aschud (not (Variables|/Script/Vehicle.CHud|GetDrawVehicleIds _aschud)))))

(fn ConstructionScript)